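; BP_CrystalGameInstance is a game instance Blueprint that holds the active save game reference and slot name.
; CreateOrLoadSaveSlot stores the given slot name, then loads an existing BP_CrystalSaveGame from that slot or creates a new one.
; A new save records its own file name and is written to the slot immediately, printing whether creation succeeded.
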(event `CreateOrLoadSaveSlot`
  (params (saveFileName :type String))
  (bind _output_get (set `self.saveFileNameGameInstance` saveFileName))
  (bind _returnvalue (`GameplayStatics.DoesSaveGameExist` _output_get))
  (if _returnvalue
    (bind _returnvalue_2 (`GameplayStatics.LoadGameFromSlot` (`self.saveFileNameGameInstance`)))
    (bind _asbp_crystal_save_game (cast `/Game/Classes/BP_CrystalSaveGame` _returnvalue_2))
    (set `self.saveGameReference` _asbp_crystal_save_game)
    (else
      (bind _returnvalue_3 (`GameplayStatics.CreateSaveGameObject` "/Game/Classes/BP_CrystalSaveGame.BP_CrystalSaveGame_C"))
      (bind _output_get_2 (set `self.saveGameReference` _returnvalue_3))
      (bind _output_get_3 (set `/Game/Classes/BP_CrystalSaveGame.saveFileName` (`self.saveFileNameGameInstance`) _output_get_2))
      (bind _returnvalue_4 (`GameplayStatics.SaveGameToSlot` _output_get_2 _output_get_3))
      (if _returnvalue_4
        (`KismetSystemLibrary.PrintString` "Save Created Successfully!")
        (else
          (`KismetSystemLibrary.PrintString` "Save Creation Failed!"))))))