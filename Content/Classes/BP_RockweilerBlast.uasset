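; BP_RockweilerBlast is an expanding blast actor that briefly knocks the crystal player out of control.
; Tick grows the actor's scale uniformly at a constant rate until it reaches MaxPushDistance.
; When BlastCollision overlaps BP_CrystalPlayer, it stores the player, disables their input and plays a roll montage.
; At maximum scale it re-enables input on the stored player, stops the montage and destroys itself.
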(event `self.BlastCollision.OnComponentBeginOverlap`
  (params (OverlappedComponent :type "PrimitiveComponent Object Reference") (OtherActor :type "Actor Object Reference") (OtherComp :type "PrimitiveComponent Object Reference") (OtherBodyIndex :type Integer) (bFromSweep :type Boolean) (SweepResult :type "HitResult Structure (by ref)"))
  (bind _asbp_crystal_player (cast `/Game/Classes/BP_CrystalPlayer` OtherActor))
  (bind _output_get (set `self.playerReference` _asbp_crystal_player))
  (`/Engine/EditorBlueprintResources/StandardMacros.IsValid` _output_get
    (:`Is Valid`
      (`self.DisableInput` _output_get null)
      (`Character.PlayAnimMontage` _output_get "/Game/Animations/Character/AM_Roll_01a.AM_Roll_01a" 1.0 "None"))))

(event `self.ReceiveTick`
  (params (DeltaSeconds :type "Float (single-precision)"))
  (bind (_returnvalue_location _returnvalue_rotation _returnvalue_scale) (`KismetMathLibrary.BreakTransform` (`self.GetTransform`)))
  (bind _returnvalue (* (`self.Delta Seconds`) 35.0))
  (set `self.Delta Seconds` DeltaSeconds)
  (if (>= (.x (.scale (`self.GetTransform`))) (`self.maxPushDistance`))
    (`self.EnableInput` (stale `self.BlastCollision.OnComponentBeginOverlap` _output_get) null)
    (`Character.StopAnimMontage` (stale `self.BlastCollision.OnComponentBeginOverlap` _output_get) "/Game/Animations/Character/AM_Roll_01a.AM_Roll_01a")
    (`self.K2_DestroyActor`)
    (else
      (`self.SetActorScale3D` (+ _returnvalue_scale (`KismetMathLibrary.MakeVector` _returnvalue _returnvalue _returnvalue))))))

(fn `UserConstructionScript`)