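; BP_MovingDeathFog is a moving hazard that kills the crystal player when the player's capsule overlaps its fog cube.
; On BeginPlay the cube snaps to StartPoint, waits a start delay, then shuttles endlessly between StartPoint and EndPoint using looped MoveComponentTo calls.
; Travel time is configurable, and optional pauses at each end apply when either endpoint delay is above zero.
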(event `self.FogCube.OnComponentBeginOverlap`
  (params (OverlappedComponent :type "PrimitiveComponent Object Reference") (OtherActor :type "Actor Object Reference") (OtherComp :type "PrimitiveComponent Object Reference") (OtherBodyIndex :type Integer) (bFromSweep :type Boolean) (SweepResult :type "HitResult Structure (by ref)"))
  (bind _asbp_crystal_player (cast `/Game/Classes/BP_CrystalPlayer` OtherActor))
  (cast `CapsuleComponent` OtherComp)
  (`/Game/Classes/BP_CrystalPlayer.Event Death` _asbp_crystal_player))

(event `self.ReceiveBeginPlay`
  (bind _travelovertime (`self.travelOverTime`))
  (bind _fogcube (`self.FogCube`))
  (bind _fogcube_2 (`self.FogCube`))
  (if (or (> (`self.endPointDelay`) 0.0) (> (`self.startPointDelay`) 0.0))
    (set `self.doesPlatformWait` true)
    (else
      (set `self.doesPlatformWait` false)))
  (set `self.platformRelativeRotation` (`SceneComponent.RelativeRotation` _fogcube))
  (`SceneComponent.K2_SetWorldLocation` _fogcube (`SceneComponent.K2_GetComponentLocation` (`self.StartPoint`)) false false)
  (`KismetSystemLibrary.Delay` (`self.movementStartDelay`))
  (`KismetSystemLibrary.MoveComponentTo` _fogcube_2 (`SceneComponent.RelativeLocation` (`self.EndPoint`)) (`self.platformRelativeRotation`) false false _travelovertime :!label _label)
  (if (`self.doesPlatformWait`)
    (`KismetSystemLibrary.Delay` (`self.endPointDelay`)))
  (`KismetSystemLibrary.MoveComponentTo` _fogcube_2 (`SceneComponent.RelativeLocation` (`self.StartPoint`)) (`self.platformRelativeRotation`) false false _travelovertime)
  (if (`self.doesPlatformWait`)
    (`KismetSystemLibrary.Delay` (`self.startPointDelay`))
    (goto _label)
    (else
      (goto _label))))

(fn `UserConstructionScript`)