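; BP_RockweilerWall is a moving wall made of a row of child actors that travels forward from its spawn point.
; The construction script spaces one child actor per column, centered across the wall width, with a random branch choosing between two child actor nodes per slot.
; Tick moves the wall horizontally along its forward vector at a fixed speed and destroys it beyond a set distance from its recorded origin.
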(event `self.ReceiveBeginPlay`
  (set `self.wallOriginPoint` (`self.K2_GetActorLocation`)))

(event `self.ReceiveTick`
  (params (DeltaSeconds :type "Float (single-precision)"))
  (bind _returnvalue (* (`self.Delta Seconds`) 2000.0))
  (set `self.Delta Seconds` DeltaSeconds)
  (`self.K2_SetActorLocation` (+ (`self.K2_GetActorLocation`) (* (`SceneComponent.GetForwardVector` (`self.DefaultSceneRoot`)) (`KismetMathLibrary.MakeVector` _returnvalue _returnvalue))))
  (if (>= (`KismetMathLibrary.Vector_Distance` (`self.K2_GetActorLocation`) (`self.wallOriginPoint`)) 10000.0)
    (`self.K2_DestroyActor`)))

(fn `UserConstructionScript`
  (locals (tempVector :type "Vector Structure") (wallWidth :type "Float (double-precision)") (columnCount :type Integer :default 16) (columnSpacing :type "Float (double-precision)" :default 275.0))
  (set `local.wallWidth` (* (`local.columnSpacing`) (`local.columnCount`)))
  (for _index (range 1 (+ (`local.columnCount`) 1))
    (if (`KismetMathLibrary.RandomBool`)
      (bind _returnvalue (`KismetMathLibrary.MapRangeUnclamped` (`KismetMathLibrary.Conv_IntToDouble` _index) 1.0 (`KismetMathLibrary.Conv_IntToDouble` (`local.columnCount`)) (/ (`local.wallWidth`) -2.0) (/ (`local.wallWidth`) 2.0)))
      (`AddComponent|NODE_AddChildActorComponent-1` :`RelativeTransform` (`KismetMathLibrary.MakeTransform` (`KismetMathLibrary.MakeVector` 0.0 _returnvalue)))
      (else
        (`AddComponent|NODE_AddChildActorComponent-2` :`RelativeTransform` (`KismetMathLibrary.MakeTransform` (`KismetMathLibrary.MakeVector` 0.0 _returnvalue)))))))