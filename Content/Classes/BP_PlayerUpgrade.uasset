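; BP_PlayerUpgrade is a one-time pickup that extends the player's slow-time duration.
; On BeginPlay it destroys itself if the save game already marks its index ID as collected, and warns if that index is invalid.
; On overlap it raises the player's clamped slow-time duration and refreshes the duration bar UI.
; It then marks itself collected, saves asynchronously and destroys itself once the save completes.
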(event `self.ReceiveBeginPlay`
  (bind _asbp_crystal_game_instance (cast `/Game/Classes/BP_CrystalGameInstance` (`GameplayStatics.GetGameInstance`)))
  (bind _upgradescollected (`/Game/Classes/BP_CrystalSaveGame.upgradesCollected` (`/Game/Classes/BP_CrystalGameInstance.saveGameReference` _asbp_crystal_game_instance)))
  (if (`KismetArrayLibrary.Array_IsValidIndex` _upgradescollected (`self.upgradeIndexID`))
    (if (== true (`|GetArrayItem` _upgradescollected (`self.upgradeIndexID`)))
      (`self.K2_DestroyActor`))
    (else
      (`KismetSystemLibrary.PrintString` "Upgrade without ID!"))))

(event `self.UpgradeCollider.OnComponentBeginOverlap`
  (params (OverlappedComponent :type "PrimitiveComponent Object Reference") (OtherActor :type "Actor Object Reference") (OtherComp :type "PrimitiveComponent Object Reference") (OtherBodyIndex :type Integer) (bFromSweep :type Boolean) (SweepResult :type "HitResult Structure (by ref)"))
  (bind _asbp_crystal_player (cast `/Game/Classes/BP_CrystalPlayer` OtherActor))
  (bind _output_get (set `/Game/Classes/BP_CrystalPlayer.currentSlowTimeDuration` (`KismetMathLibrary.FClamp` (+ (`/Game/Classes/BP_CrystalPlayer.currentSlowTimeDuration` _asbp_crystal_player) (`/Game/Classes/BP_CrystalPlayer.slowTimeUpgradeIncrementValue` _asbp_crystal_player)) (`/Game/Classes/BP_CrystalPlayer.defaultSlowTimeDuration` _asbp_crystal_player) (`/Game/Classes/BP_CrystalPlayer.maxSlowTimeDuration` _asbp_crystal_player)) _asbp_crystal_player))
  (`KismetSystemLibrary.PrintString` (`KismetStringLibrary.Conv_DoubleToString` _output_get))
  (`/Game/Classes/BP_CrystalPlayer.UpdateUICrystalClarityDurationBar` _asbp_crystal_player)
  (bind _asbp_crystal_game_instance (cast `/Game/Classes/BP_CrystalGameInstance` (`GameplayStatics.GetGameInstance`)))
  (bind _savegamereference (`/Game/Classes/BP_CrystalGameInstance.saveGameReference` _asbp_crystal_game_instance))
  (`KismetArrayLibrary.Array_Set` (`/Game/Classes/BP_CrystalSaveGame.upgradesCollected` _savegamereference) (`self.upgradeIndexID`) true)
  (`AsyncActionHandleSaveGame.AsyncSaveGameToSlot` _savegamereference (`/Game/Classes/BP_CrystalSaveGame.saveFileName` _savegamereference)
    (:`Completed`
      (`KismetSystemLibrary.PrintString` "Save done!")
      (`self.K2_DestroyActor`))))

(fn `UserConstructionScript`)