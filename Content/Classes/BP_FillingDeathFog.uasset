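; BP_FillingDeathFog is a hazard volume that fills and drains between StartPoint and EndPoint, killing the crystal player on contact.
; Two timelines, rate-scaled by FillVelocity over distance, stretch and move FogCube while raising FogTop.
; Segments chain through FogTop overlaps with other fogs, with first and last flags handling delayed starts and reversals.
; An optional trigger box resets the fog when the player enters it.
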(event `self.FogCube.OnComponentBeginOverlap`
  (params (OverlappedComponent :type "PrimitiveComponent Object Reference") (OtherActor :type "Actor Object Reference") (OtherComp :type "PrimitiveComponent Object Reference") (OtherBodyIndex :type Integer) (bFromSweep :type Boolean) (SweepResult :type "HitResult Structure (by ref)"))
  (bind _asbp_crystal_player (cast `/Game/Classes/BP_CrystalPlayer` OtherActor))
  (cast `CapsuleComponent` OtherComp)
  (`/Game/Classes/BP_CrystalPlayer.Event Death` _asbp_crystal_player))

(event `ResetFogFlow`
  (`KismetSystemLibrary.Delay` (`self.movementStartDelay`) :!label _label)
  (if (`self.isFirstFogOfFill`)
    (`PrimitiveComponent.SetCollisionEnabled` (`self.FogCube`) "QueryOnly")
    (`self.ChangeFogFill` true)))

(event `self.ReceiveBeginPlay`
  (bind _fogtop (`self.FogTop`))
  (bind _fogcube (`self.FogCube`))
  (bind (_returnvalue_x _returnvalue_y) (`KismetMathLibrary.BreakVector` (`SceneComponent.K2_GetComponentScale` (`self.FogCube`))))
  (bind (_returnvalue_x_2 _returnvalue_y_2 _returnvalue_z) (`KismetMathLibrary.BreakVector` (`SceneComponent.K2_GetComponentLocation` (`self.FogCube`))))
  (bind (_returnvalue_x_3 _returnvalue_y_3) (`KismetMathLibrary.BreakVector` (`SceneComponent.K2_GetComponentScale` _fogcube)))
  (if (not (`self.hasResetTriggerBox`))
    (`PrimitiveComponent.SetCollisionEnabled` (`self.ResetTriggerBox`) "NoCollision"))
  (`SceneComponent.SetWorldScale3D` _fogcube (`KismetMathLibrary.MakeVector` _returnvalue_x_3 _returnvalue_y_3))
  (`SceneComponent.K2_SetWorldLocation` _fogcube (`SceneComponent.K2_GetComponentLocation` (`self.StartPoint`)) false false)
  (`SceneComponent.SetWorldScale3D` _fogtop (`KismetMathLibrary.MakeVector` _returnvalue_x _returnvalue_y 0.1))
  (bind _output_get (set `self.fogTopStartPoint` (`KismetMathLibrary.MakeVector` _returnvalue_x_2 _returnvalue_y_2 (+ _returnvalue_z 1.0))))
  (`SceneComponent.K2_SetWorldLocation` _fogtop _output_get false false)
  (`PrimitiveComponent.SetCollisionEnabled` (`self.FogCube`) "NoCollision")
  (goto _label))

(event `self.FogTop.OnComponentBeginOverlap`
  (params (OverlappedComponent :type "PrimitiveComponent Object Reference") (OtherActor :type "Actor Object Reference") (OtherComp :type "PrimitiveComponent Object Reference") (OtherBodyIndex :type Integer) (bFromSweep :type Boolean) (SweepResult :type "HitResult Structure (by ref)"))
  (cast `/Game/Classes/BP_FillingDeathFog` OtherActor)
  (cast `BoxComponent` OtherComp)
  (`/Engine/EditorBlueprintResources/StandardMacros.DoOnce` false :!label _label_2
    (:`Completed`
      (`self.ChangeFogFill` (`self.isFillingUp`))
      (`PrimitiveComponent.SetCollisionEnabled` (`self.FogCube`) "QueryOnly"))))

(event `ResetFogTopDetection`
  (`KismetSystemLibrary.DelayUntilNextTick`)
  (goto _label_2 :!via `Reset`))

(event `ChangeFogFillEvent`
  (bind (_fogtopstartpoint_x _fogtopstartpoint_y _fogtopstartpoint_z) (`KismetMathLibrary.BreakVector` (`self.fogTopStartPoint`)))
  (bind (_returnvalue_x _returnvalue_y) (`KismetMathLibrary.BreakVector` (`SceneComponent.K2_GetComponentScale` (`self.FogCube`))))
  (bind (_returnvalue_x_2 _returnvalue_y_2 _returnvalue_z) (`KismetMathLibrary.BreakVector` (`SceneComponent.K2_GetComponentLocation` (`self.StartPoint`))))
  (bind _returnvalue (`KismetMathLibrary.Vector_Distance` (`SceneComponent.RelativeLocation` (`self.StartPoint`)) (`SceneComponent.RelativeLocation` (`self.EndPoint`))))
  (`|ExecutionSequence`
    (:`then_0`
      (`TimelineComponent.SetPlayRate` (`self.FogCubeGrowthTimeline`) (/ (`self.fillVelocity`) _returnvalue))
      (if (`self.isFillingUp`)
        (bind (_direction _newtrack_0) (`Timeline|FogCubeGrowthTimeline` :!label _label_3)
          (:`Update`
            (`SceneComponent.SetWorldScale3D` (`self.FogCube`) (* (`KismetMathLibrary.MakeVector` 1.0 1.0 _newtrack_0) (`KismetMathLibrary.MakeVector` _returnvalue_x _returnvalue_y (/ _returnvalue 100.0))))))
        (else
          (goto _label_3 :!via `Reverse`))))
    (:`then_1`
      (`TimelineComponent.SetPlayRate` (`self.FogMovementTimeline`) (/ (`self.fillVelocity`) (`KismetMathLibrary.Vector_Distance` (`SceneComponent.RelativeLocation` (`self.StartPoint`)) (`SceneComponent.RelativeLocation` (`self.EndPoint`)))))
      (if (`self.isFillingUp`)
        (bind (_direction_2 _fogmovementtrack) (`Timeline|FogMovementTimeline` :!label _label_4)
          (:`Update`
            (`|ExecutionSequence`
              (:`then_0`
                (bind _returnvalue_2 (* _fogmovementtrack (`KismetMathLibrary.Vector_Distance` (`SceneComponent.RelativeLocation` (`self.StartPoint`)) (`SceneComponent.RelativeLocation` (`self.EndPoint`)))))
                (`SceneComponent.K2_SetWorldLocation` (`self.FogCube`) (`KismetMathLibrary.MakeVector` _returnvalue_x_2 _returnvalue_y_2 (+ _returnvalue_z (/ _returnvalue_2 2.0))) false false))
              (:`then_1`
                (`SceneComponent.K2_SetWorldLocation` (`self.FogTop`) (`KismetMathLibrary.MakeVector` _fogtopstartpoint_x _fogtopstartpoint_y (+ _fogtopstartpoint_z _returnvalue_2)) false false))))
          (:`Finished`
            (`self.FogFillFinish`)))
        (else
          (goto _label_4 :!via `Reverse`))))))

(event `ResetFogGrowth`
  (`|ExecutionSequence`
    (:`then_0`
      (goto _label_3 :!via `Stop`))
    (:`then_1`
      (goto _label_3 :!via `SetNewTime`))))

(event `ResetFogPosition`
  (`|ExecutionSequence`
    (:`then_0`
      (goto _label_4 :!via `Stop`))
    (:`then_1`
      (goto _label_4 :!via `SetNewTime`))
    (:`then_2`
      (`self.ResetFogFlow`))))

(event `FogFillFinish`
  (if (`self.isFirstFogOfFill`)
    (if (`self.isFillingUp`)
      (set `self.isFillingUp` false)
      (`self.ResetFogTopDetection`)
      (else
        (`PrimitiveComponent.SetCollisionEnabled` (`self.FogCube`) "NoCollision")
        (`KismetSystemLibrary.Delay` (`self.startPointDelay`))
        (`PrimitiveComponent.SetCollisionEnabled` (`self.FogCube`) "QueryOnly")
        (`self.ChangeFogFill` true)))
    (elif (`self.isLastFogOfFill`)
      (if (`self.isFillingUp`)
        (`self.ResetFogTopDetection`)
        (if (> (`self.endPointDelay`) 0.0)
          (`KismetSystemLibrary.Delay` (`self.endPointDelay`)))
        (`self.ChangeFogFill` false)
        (else
          (set `self.isFillingUp` true)
          (`self.ResetFogTopDetection`)
          (`PrimitiveComponent.SetCollisionEnabled` (`self.FogCube`) "NoCollision")))
      (elif (`self.isFillingUp`)
        (`KismetSystemLibrary.DelayUntilNextTick`)
        (set `self.isFillingUp` false)
        (`self.ResetFogTopDetection`)
        (else
          (`KismetSystemLibrary.DelayUntilNextTick`)
          (set `self.isFillingUp` true)
          (`self.ResetFogTopDetection`)
          (`PrimitiveComponent.SetCollisionEnabled` (`self.FogCube`) "NoCollision"))))))

(event `self.ResetTriggerBox.OnComponentBeginOverlap`
  (params (OverlappedComponent :type "PrimitiveComponent Object Reference") (OtherActor :type "Actor Object Reference") (OtherComp :type "PrimitiveComponent Object Reference") (OtherBodyIndex :type Integer) (bFromSweep :type Boolean) (SweepResult :type "HitResult Structure (by ref)"))
  (cast `/Game/Classes/BP_CrystalPlayer` OtherActor)
  (cast `CapsuleComponent` OtherComp)
  (`self.ResetFogGrowth`)
  (`self.ResetFogPosition`)
  (`PrimitiveComponent.SetCollisionEnabled` (`self.FogCube`) "NoCollision")
  (`self.ResetFogTopDetection`)
  (`KismetSystemLibrary.PrintString` "Reset Fog" true true (struct :`G` 0.66 :`B` 1.0 :`A` 1.0) 5.0))

(fn `ChangeFogFill`
  (params (isFillingUp :type Boolean))
  (set `self.isFillingUp` isFillingUp)
  (`self.ChangeFogFillEvent`))

(fn `UserConstructionScript`)