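; Game mode for the crystal game that restores saved progress when play begins and controls pausing.
; BeginPlay reads the game instance's save to count collected shards, teleport the player to the last checkpoint and rebuild slow-time duration from collected upgrades, clamped to a maximum.
; It then creates the player HUD, refreshes its displays and binds PauseControl.
; PauseControl flip-flops the pause menu, game pause, input mode and mouse cursor, reusing one menu widget.
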(event `self.ReceiveBeginPlay`
  (bind _gamemodeplayercharreference (`self.gameModePlayerCharReference`))
  (bind _gamemodeplayercharreference_2 (`self.gameModePlayerCharReference`))
  (bind _lastcheckpointsaved (`/Game/Classes/BP_CrystalSaveGame.lastCheckpointSaved` (`self.gameModeSaveGameReference`)))
  (bind _asbp_crystal_player (cast `/Game/Classes/BP_CrystalPlayer` (`GameplayStatics.GetPlayerCharacter` 0)))
  (set `self.gameModePlayerCharReference` _asbp_crystal_player)
  (bind _asbp_crystal_game_instance (cast `/Game/Classes/BP_CrystalGameInstance` (`GameplayStatics.GetGameInstance`)))
  (bind _output_get (set `self.gameModeSaveGameReference` (`/Game/Classes/BP_CrystalGameInstance.saveGameReference` _asbp_crystal_game_instance)))
  (for _array_element (`/Game/Classes/BP_CrystalSaveGame.shardsCollected` _output_get)
    (if _array_element
      (`/Engine/EditorBlueprintResources/StandardMacros.IncrementInt` (`self.collectedCrystalShards`))))
  (if (`/Game/Classes/BP_CrystalSaveGame.hasReachedFirstCheckpoint` (`self.gameModeSaveGameReference`))
    (set `/Game/Classes/BP_CrystalPlayer.lastCheckpoint` _lastcheckpointsaved (`self.gameModePlayerCharReference`))
    (`self.K2_SetActorTransform` (`GameplayStatics.GetPlayerCharacter` 0) _lastcheckpointsaved false false)
    (else
      (set `/Game/Classes/BP_CrystalPlayer.lastCheckpoint` (`self.GetTransform` (`GameplayStatics.GetPlayerCharacter` 0)) (`self.gameModePlayerCharReference`))))
  (set `/Game/Classes/BP_CrystalPlayer.currentSlowTimeDuration` (`/Game/Classes/BP_CrystalPlayer.defaultSlowTimeDuration` _gamemodeplayercharreference) _gamemodeplayercharreference)
  (for _array_element_2 (`/Game/Classes/BP_CrystalSaveGame.upgradesCollected` (`self.gameModeSaveGameReference`))
    (if _array_element_2
      (set `/Game/Classes/BP_CrystalPlayer.currentSlowTimeDuration` (`KismetMathLibrary.FClamp` (+ (`/Game/Classes/BP_CrystalPlayer.currentSlowTimeDuration` _gamemodeplayercharreference_2) (`/Game/Classes/BP_CrystalPlayer.slowTimeUpgradeIncrementValue` _gamemodeplayercharreference_2)) (`/Game/Classes/BP_CrystalPlayer.defaultSlowTimeDuration` _gamemodeplayercharreference_2) (`/Game/Classes/BP_CrystalPlayer.maxSlowTimeDuration` _gamemodeplayercharreference_2)) _gamemodeplayercharreference_2)))
  (bind _returnvalue (`|CreateWidget` "/Game/UI/UIBP_CrystalPlayerHUD.UIBP_CrystalPlayerHUD_C" (`GameplayStatics.GetPlayerController` 0)))
  (`UserWidget.AddToViewport` _returnvalue 0)
  (`/Game/Classes/BP_CrystalPlayer.UpdateUICrystalClarityDurationBar` (`self.gameModePlayerCharReference`))
  (`self.UpdateShardCounter`)
  (add `self.PauseController` (delegate `PauseControl`)))

(event `PauseControl`
  (bind _returnvalue (`GameplayStatics.GetPlayerController` 0))
  (bind _returnvalue_2 (`GameplayStatics.GetPlayerController` 0))
  (`/Engine/EditorBlueprintResources/StandardMacros.FlipFlop`
    (:`A`
      (`GameplayStatics.SetGamePaused` true)
      (set `self.isPaused` true)
      (`/Engine/EditorBlueprintResources/StandardMacros.IsValid` (`self.pauseMenu`)
        (:`Is Valid`
          _)
        (:`Is Not Valid`
          (bind _returnvalue_3 (`|CreateWidget` "/Game/UI/UIBP_PauseMenu.UIBP_PauseMenu_C"))
          (set `self.pauseMenu` _returnvalue_3)))
      (`UserWidget.AddToViewport` (`self.pauseMenu`) 0)
      (`WidgetBlueprintLibrary.SetInputMode_GameAndUIEx` _returnvalue_2 null)
      (set `PlayerController.bShowMouseCursor` true _returnvalue_2))
    (:`B`
      (`Widget.RemoveFromParent` (`self.pauseMenu`))
      (`WidgetBlueprintLibrary.SetInputMode_GameOnly` _returnvalue)
      (set `PlayerController.bShowMouseCursor` false _returnvalue)
      (`GameplayStatics.SetGamePaused` false)
      (set `self.isPaused` false))))

(fn `UserConstructionScript`)