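; Manager that cycles a network of filling death fogs up and down after an initial delay.
; A timeline, with play rate scaled from fill velocity and start-to-end distance, moves a height indicator vertically from the start point.
; Each direction change is passed to all referenced fogs, with optional pauses at either end.
; ResetFogNetwork resets the timeline and every fog, then restarts the cycle.
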(event `ResetFogFlow`
  (`KismetSystemLibrary.Delay` (`self.movementStartDelay`) :!label _label)
  (`self.ChangeFogFillDirection` true))

(event `self.ReceiveBeginPlay`
  (goto _label))

(event `ChangeFogFillDirectionEvent`
  (bind (_returnvalue_x _returnvalue_y _returnvalue_z) (`KismetMathLibrary.BreakVector` (`SceneComponent.K2_GetComponentLocation` (`self.StartPoint`))))
  (`TimelineComponent.SetPlayRate` (`self.FogMovementTimeline`) (/ (`self.fillVelocity`) (`KismetMathLibrary.Vector_Distance` (`SceneComponent.RelativeLocation` (`self.StartPoint`)) (`SceneComponent.RelativeLocation` (`self.EndPoint`)))))
  (if (`self.isFillingUp`)
    (bind (_direction _fogmovementtrack) (`Timeline|FogMovementTimeline` :!label _label_2)
      (:`Update`
        (`SceneComponent.K2_SetWorldLocation` (`self.FogHeightIndicator`) (`KismetMathLibrary.MakeVector` _returnvalue_x _returnvalue_y (+ _returnvalue_z (* _fogmovementtrack (`KismetMathLibrary.Vector_Distance` (`SceneComponent.RelativeLocation` (`self.StartPoint`)) (`SceneComponent.RelativeLocation` (`self.EndPoint`)))))) false false))
      (:`Finished`
        (`self.FogFillFinish`)))
    (else
      (goto _label_2 :!via `Reverse`))))

(event `ResetFogPosition`
  (`|ExecutionSequence`
    (:`then_0`
      (goto _label_2 :!via `Stop`))
    (:`then_1`
      (goto _label_2 :!via `SetNewTime`))
    (:`then_2`
      (`self.ResetFogFlow`))))

(event `FogFillFinish`
  (if (`self.isFillingUp`)
    (if (> (`self.endPointDelay`) 0.0)
      (`KismetSystemLibrary.Delay` (`self.endPointDelay`)))
    (`self.ChangeFogFillDirection` false)
    (else
      (if (> (`self.startPointDelay`) 0.0)
        (`KismetSystemLibrary.Delay` (`self.startPointDelay`)))
      (`self.ChangeFogFillDirection` true))))

(fn `ChangeFogFillDirection`
  (params (isFillingUp :type Boolean))
  (bind _output_get (set `self.isFillingUp` isFillingUp))
  (for _array_element (`self.fillingFogReferenceArray`)
    (`/Game/Classes/BP_FillingDeathFog.SetFogDirection` _array_element _output_get))
  (`self.ChangeFogFillDirectionEvent`))

(fn `ResetFogNetwork`
  (`self.ResetFogPosition`)
  (set `self.isFillingUp` true)
  (for _array_element (`self.fillingFogReferenceArray`)
    (`/Game/Classes/BP_FillingDeathFog.ResetFog` _array_element))
  (`self.ResetFogFlow`)
  (`KismetSystemLibrary.PrintString` "Fog Reset."))

(fn `UserConstructionScript`)