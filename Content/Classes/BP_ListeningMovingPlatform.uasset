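; A moving platform Blueprint that makes a round trip between start and end points when its MovePlatform event fires.
; BeginPlay stores the platform collision's relative rotation and snaps it to the start point.
; MovePlatform uses MoveComponentTo to glide it to the end point over a set travel time, waits a delay, then glides it back, keeping the stored rotation.
; Nothing in this graph calls MovePlatform, so an external trigger must fire it.
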(event `Move Platform`
  (bind _travelovertime (`self.travelOverTime`))
  (bind _platformcollisiontop (`self.PlatformCollisionTop`))
  (`KismetSystemLibrary.MoveComponentTo` _platformcollisiontop (`SceneComponent.RelativeLocation` (`self.EndPoint`)) (`self.platformRelativeRotation`) false false _travelovertime)
  (`KismetSystemLibrary.Delay` (`self.endPointDelay`))
  (`KismetSystemLibrary.MoveComponentTo` _platformcollisiontop (`SceneComponent.RelativeLocation` (`self.StartPoint`)) (`self.platformRelativeRotation`) false false _travelovertime))

(event `self.ReceiveBeginPlay`
  (set `self.platformRelativeRotation` (`SceneComponent.RelativeRotation` (`self.PlatformCollisionTop`)))
  (`SceneComponent.K2_SetWorldLocation` (`self.PlatformCollisionTop`) (`SceneComponent.K2_GetComponentLocation` (`self.StartPoint`)) false false))

(fn `UserConstructionScript`)