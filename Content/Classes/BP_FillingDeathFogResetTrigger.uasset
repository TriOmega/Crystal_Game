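; Trigger actor that resets the filling death fog when the crystal player enters it.
; An overlap by the BP_CrystalPlayer's capsule component on the ResetTrigger volume calls ResetFogNetwork on the referenced fog manager.
; On BeginPlay it prints an on-screen warning if that manager reference is invalid.
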(event `self.ReceiveBeginPlay`
  (if (not (`KismetSystemLibrary.IsValid` (`self.fogManagerReference`)))
    (`KismetSystemLibrary.PrintString` (`KismetStringLibrary.Concat_StrStr` (`KismetSystemLibrary.GetDisplayName` self) " has invalid manager reference!") true true (struct :`G` 0.66 :`B` 1.0 :`A` 1.0) 4.0)))

(event `self.ResetTrigger.OnComponentBeginOverlap`
  (params (OverlappedComponent :type "PrimitiveComponent Object Reference") (OtherActor :type "Actor Object Reference") (OtherComp :type "PrimitiveComponent Object Reference") (OtherBodyIndex :type Integer) (bFromSweep :type Boolean) (SweepResult :type "HitResult Structure (by ref)"))
  (cast `/Game/Classes/BP_CrystalPlayer` OtherActor)
  (cast `CapsuleComponent` OtherComp)
  (`/Game/Classes/BP_FillingDeathFogManager.ResetFogNetwork` (`self.fogManagerReference`)))

(fn `UserConstructionScript`)