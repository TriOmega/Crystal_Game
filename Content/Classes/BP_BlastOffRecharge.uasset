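; Blast-off recharge crystal pickup that restores the crystal player's abilities when touched.
; On overlap it readies Blast Off, clears the launched state, completes the Crystal Clarity cooldown with a UI update, and triggers the player's slow-time event, passing its own class.
; It then hides its mesh and disables collision, re-enabling both after a respawn delay.
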(event `self.RechargeCollision.OnComponentBeginOverlap`
  (params (OverlappedComponent :type "PrimitiveComponent Object Reference") (OtherActor :type "Actor Object Reference") (OtherComp :type "PrimitiveComponent Object Reference") (OtherBodyIndex :type Integer) (bFromSweep :type Boolean) (SweepResult :type "HitResult Structure (by ref)"))
  (bind _asbp_crystal_player (cast `/Game/Classes/BP_CrystalPlayer` OtherActor))
  (`/Engine/EditorBlueprintResources/StandardMacros.IsValid` _asbp_crystal_player
    (:`Is Valid`
      (set `/Game/Classes/BP_CrystalPlayer.isLaunched` false _asbp_crystal_player)
      (set `/Game/Classes/BP_CrystalPlayer.isBlastOffReady` true _asbp_crystal_player)
      (set `/Game/Classes/BP_CrystalPlayer.isCrystalClarityCooldownDone` true _asbp_crystal_player)
      (set `/Game/Classes/BP_CrystalPlayer.crystalClarityCooldownDurationRemainder` (`/Game/Classes/BP_CrystalPlayer.crystalClarityCooldownDuration` _asbp_crystal_player) _asbp_crystal_player)
      (`/Game/Classes/BP_CrystalPlayer.UpdateUICrystalClarityCooldown` _asbp_crystal_player)
      (`SceneComponent.SetVisibility` (`self.RechargeCrystalMesh`) false false)
      (`PrimitiveComponent.SetCollisionEnabled` (`self.RechargeCollision`) "NoCollision")
      (`/Game/Classes/BP_CrystalPlayer.Event Begin Slow Time` _asbp_crystal_player (`GameplayStatics.GetObjectClass` self))
      (`KismetSystemLibrary.Delay` (`self.rechargeRespawnDuration`))
      (`SceneComponent.SetVisibility` (`self.RechargeCrystalMesh`) true false)
      (`PrimitiveComponent.SetCollisionEnabled` (`self.RechargeCollision`) "QueryAndPhysics"))))

(fn `UserConstructionScript`)