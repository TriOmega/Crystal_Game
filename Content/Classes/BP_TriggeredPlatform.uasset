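; A triggered platform that moves from start to end point when the player touches its crystal trigger, serving as a reusable lift or one-time door.
; Reusable platforms return after a delay or when a reset trigger is overlapped, with a gate blocking the timed return after a manual reset.
; One-time platforms save their opened state by index in the game mode's save, then restore it on BeginPlay, destroying unneeded triggers.
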(event `self.ReceiveBeginPlay`
  (bind _onetimedoorindex (`self.oneTimeDoorIndex`))
  (bind _onetimedoorsopened (`/Game/Classes/BP_CrystalSaveGame.oneTimeDoorsOpened` (`/Game/Classes/BP_CrystalGameMode.gameModeSaveGameReference` (`self.gameModeReference`))))
  (set `self.platformRelativeRotation` (`SceneComponent.RelativeRotation` (`self.PlatformCollisionTop`)))
  (`KismetSystemLibrary.Delay` 2.0)
  (bind _asbp_crystal_game_mode (cast `/Game/Classes/BP_CrystalGameMode` (`GameplayStatics.GetGameMode`)))
  (set `self.gameModeReference` _asbp_crystal_game_mode)
  (if (`self.isOneTimeUse`)
    (if (`KismetArrayLibrary.Array_IsValidIndex` _onetimedoorsopened _onetimedoorindex)
      (if (== (`|GetArrayItem` _onetimedoorsopened _onetimedoorindex) true)
        (`SceneComponent.K2_SetWorldLocation` (`self.PlatformCollisionTop`) (`SceneComponent.K2_GetComponentLocation` (`self.EndPoint`)) false false)
        (`ActorComponent.K2_DestroyComponent` (`self.ExtraResetTrigger`))
        (`ActorComponent.K2_DestroyComponent` (`self.PlatformResetTrigger`))
        (`ActorComponent.K2_DestroyComponent` (`self.ResetTriggerCrystalMesh`))
        (`ActorComponent.K2_DestroyComponent` (`self.PlatformTrigger`))
        (`ActorComponent.K2_DestroyComponent` (`self.TriggerCrystalMesh`))
        (else
          (`ActorComponent.K2_DestroyComponent` (`self.ExtraResetTrigger`))
          (`ActorComponent.K2_DestroyComponent` (`self.PlatformResetTrigger`))
          (`ActorComponent.K2_DestroyComponent` (`self.ResetTriggerCrystalMesh`))
          (`SceneComponent.K2_SetWorldLocation` (`self.PlatformCollisionTop`) (`SceneComponent.K2_GetComponentLocation` (`self.StartPoint`)) false false :!label _label)
          (`SceneComponent.SetVisibility` (`self.ResetTriggerCrystalMesh`) false false)
          (if (`self.hasExtraTrigger`)
            (set `PrimitiveComponent.bGenerateOverlapEvents` true (`self.ExtraResetTrigger`))
            (else
              (set `PrimitiveComponent.bGenerateOverlapEvents` false (`self.ExtraResetTrigger`))))))
      (else
        (`KismetSystemLibrary.PrintString` "One Time Door without valid ID!")))
    (else
      (goto _label))))

(event `self.PlatformTrigger.OnComponentBeginOverlap`
  (params (OverlappedComponent :type "PrimitiveComponent Object Reference") (OtherActor :type "Actor Object Reference") (OtherComp :type "PrimitiveComponent Object Reference") (OtherBodyIndex :type Integer) (bFromSweep :type Boolean) (SweepResult :type "HitResult Structure (by ref)"))
  (bind _platformcollisiontop (`self.PlatformCollisionTop`))
  (bind _gamemodesavegamereference (`/Game/Classes/BP_CrystalGameMode.gameModeSaveGameReference` (`self.gameModeReference`)))
  (cast `/Game/Classes/BP_CrystalPlayer` OtherActor)
  (if (`self.isOneTimeUse`)
    (`KismetArrayLibrary.Array_Set` (`/Game/Classes/BP_CrystalSaveGame.oneTimeDoorsOpened` _gamemodesavegamereference) (`self.oneTimeDoorIndex`) true)
    (`AsyncActionHandleSaveGame.AsyncSaveGameToSlot` _gamemodesavegamereference (`/Game/Classes/BP_CrystalSaveGame.saveFileName` _gamemodesavegamereference)
      (:`then`
        _)))
  (set `PrimitiveComponent.bGenerateOverlapEvents` false (`self.PlatformTrigger`))
  (`SceneComponent.SetVisibility` (`self.TriggerCrystalMesh`) false false)
  (`KismetSystemLibrary.MoveComponentTo` _platformcollisiontop (`SceneComponent.RelativeLocation` (`self.EndPoint`)) (`self.platformRelativeRotation`) false false (`self.destinationTravelTime`))
  (if (`self.isOneTimeUse`)
    (`ActorComponent.K2_DestroyComponent` (`self.PlatformTrigger`))
    (`ActorComponent.K2_DestroyComponent` (`self.TriggerCrystalMesh`))
    (else
      (`self.ActivateResetTrigger`)
      (`KismetSystemLibrary.Delay` (`self.endPointDelay`))
      (`SceneComponent.SetVisibility` (`self.ResetTriggerCrystalMesh`) false false)
      (set `PrimitiveComponent.bGenerateOverlapEvents` false (`self.PlatformResetTrigger`))
      (`/Engine/EditorBlueprintResources/StandardMacros.Gate` false :!label _label_2
        (:`Exit`
          (`KismetSystemLibrary.MoveComponentTo` _platformcollisiontop (`SceneComponent.RelativeLocation` (`self.StartPoint`)) (`self.platformRelativeRotation`) false false (`self.resetTravelTime`) :!label _label_3)
          (`SceneComponent.SetVisibility` (`self.ResetTriggerCrystalMesh`) false false)
          (set `PrimitiveComponent.bGenerateOverlapEvents` false (`self.PlatformResetTrigger`))
          (if (`self.hasExtraDelayOnReset`)
            (`KismetSystemLibrary.Delay` 4.0))
          (`SceneComponent.SetVisibility` (`self.TriggerCrystalMesh`) true false)
          (set `PrimitiveComponent.bGenerateOverlapEvents` true (`self.PlatformTrigger`))
          (`KismetSystemLibrary.Delay` (`self.resetTravelTime`))
          (goto _label_2 :!via `Open`))))))

(event `ActivateResetTrigger`
  (`SceneComponent.SetVisibility` (`self.ResetTriggerCrystalMesh`) true false)
  (set `PrimitiveComponent.bGenerateOverlapEvents` true (`self.PlatformResetTrigger`)))

(event `self.PlatformResetTrigger.OnComponentBeginOverlap`
  (params (OverlappedComponent :type "PrimitiveComponent Object Reference") (OtherActor :type "Actor Object Reference") (OtherComp :type "PrimitiveComponent Object Reference") (OtherBodyIndex :type Integer) (bFromSweep :type Boolean) (SweepResult :type "HitResult Structure (by ref)"))
  (bind _gamemodehudreference (`/Game/Classes/BP_CrystalGameMode.gameModeHUDReference` (`self.gameModeReference`)))
  (`SceneComponent.SetVisibility` (`self.ResetTriggerCrystalMesh`) false false :!label _label_4)
  (set `PrimitiveComponent.bGenerateOverlapEvents` false (`self.PlatformResetTrigger`))
  (`|ExecutionSequence`
    (:`then_0`
      (goto _label_2 :!via `Close`))
    (:`then_1`
      (goto _label_3))
    (:`then_2`
      (`/Game/UI/UIBP_CrystalPlayerHUD.ShowMessagePrompt` _gamemodehudreference "Platform Reset")
      (`KismetSystemLibrary.Delay` 5.0)
      (`/Game/UI/UIBP_CrystalPlayerHUD.HideMessagePrompt` _gamemodehudreference))))

(event `self.ExtraResetTrigger.OnComponentBeginOverlap`
  (params (OverlappedComponent :type "PrimitiveComponent Object Reference") (OtherActor :type "Actor Object Reference") (OtherComp :type "PrimitiveComponent Object Reference") (OtherBodyIndex :type Integer) (bFromSweep :type Boolean) (SweepResult :type "HitResult Structure (by ref)"))
  (goto _label_4))

(fn `UserConstructionScript`)