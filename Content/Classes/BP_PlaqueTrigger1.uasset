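; BP_PlaqueTrigger1 is a box trigger that gates game completion on collecting the 20 shards of the Door of Clarity.
; On overlap, unless the save game marks the game completed, it counts collected shards in the save data held by BP_CrystalGameMode.
; With enough shards it pauses the game and shows the win screen with cursor and sound.
; Otherwise it shows a timed HUD hint to collect them all.
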(event `self.BoxCollision.OnComponentBeginOverlap`
  (params (OverlappedComponent :type "PrimitiveComponent Object Reference") (OtherActor :type "Actor Object Reference") (OtherComp :type "PrimitiveComponent Object Reference") (OtherBodyIndex :type Integer) (bFromSweep :type Boolean) (SweepResult :type "HitResult Structure (by ref)"))
  (bind _returnvalue (`GameplayStatics.GetPlayerController` 0))
  (bind _asbp_crystal_game_mode (cast `/Game/Classes/BP_CrystalGameMode` (`GameplayStatics.GetGameMode`)))
  (bind _gamemodesavegamereference (`/Game/Classes/BP_CrystalGameMode.gameModeSaveGameReference` _asbp_crystal_game_mode))
  (if (not (`/Game/Classes/BP_CrystalSaveGame.hasCompletedGame` _gamemodesavegamereference))
    (set `self.shardCount` 0)
    (for _array_element (`/Game/Classes/BP_CrystalSaveGame.shardsCollected` _gamemodesavegamereference)
      (if _array_element
        (`/Engine/EditorBlueprintResources/StandardMacros.IncrementInt` (`self.shardCount`))))
    (if (>= (`self.shardCount`) 20)
      (`GameplayStatics.SetGamePaused` true)
      (bind _returnvalue_2 (`|CreateWidget` "/Game/UI/UIBP_WinScreen.UIBP_WinScreen_C"))
      (`UserWidget.AddToViewport` _returnvalue_2 0)
      (`WidgetBlueprintLibrary.SetInputMode_GameAndUIEx` _returnvalue null)
      (set `PlayerController.bShowMouseCursor` true _returnvalue)
      (`GameplayStatics.PlaySound2D` "/Game/Audio/SFX_WinScreen_01a.SFX_WinScreen_01a" 1.0 1.0 0.0 null null)
      (else
        (bind _gamemodehudreference (`/Game/Classes/BP_CrystalGameMode.gameModeHUDReference` _asbp_crystal_game_mode))
        (`/Game/UI/UIBP_CrystalPlayerHUD.ShowMessagePrompt` :`self` _gamemodehudreference :`MessageToShow` "Only those with the power of Crystal Clarity shall overcome this trial. Retrieve all 20 shards of the Door of Clarity to prove your mastery.")
        (`KismetSystemLibrary.Delay` 15.0)
        (`/Game/UI/UIBP_CrystalPlayerHUD.HideMessagePrompt` _gamemodehudreference)))))

(fn `UserConstructionScript`)