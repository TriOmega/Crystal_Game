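; BP_RotatingPlatform is a platform actor that spins continuously through its RotatingMovement component.
; BeginPlay builds the component's rotation rate from separate roll, pitch and yaw rate variables.
; When IsTrackingRotationTime is set, Tick accumulates elapsed time, then prints and resets it whenever the actor's yaw nears a fixed reference angle, as a debug timer for rotation duration.
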(event `self.ReceiveBeginPlay`
  (set `RotatingMovementComponent.RotationRate` (`KismetMathLibrary.MakeRotator` (`self.rotationRateXRoll`) (`self.rotationRateYPitch`) (`self.rotationRateZYaw`)) (`self.RotatingMovement`)))

(event `self.ReceiveTick`
  (params (DeltaSeconds :type "Float (single-precision)"))
  (bind (_returnvalue_roll _returnvalue_pitch _returnvalue_yaw) (`KismetMathLibrary.BreakRotator` (`self.K2_GetActorRotation`)))
  (if (`self.isTrackingRotationTime`)
    (set `self.singleRotationTime` (+ DeltaSeconds (`self.singleRotationTime`)))
    (if (`KismetMathLibrary.NearlyEqual_FloatFloat` _returnvalue_yaw -150.0 1.0)
      (`KismetSystemLibrary.PrintString` (`KismetStringLibrary.Conv_DoubleToString` (`self.singleRotationTime`)))
      (set `self.singleRotationTime` 0.0))))

(fn `UserConstructionScript`)