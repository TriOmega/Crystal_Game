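; BP_TestingTeleporter is a two-way teleporter that moves the BP_CrystalPlayer between two collision volumes within the same actor.
; Overlapping either volume with the player's capsule component sets the player's transform to the other volume's world location and rotation.
; A shared CanTeleportersBeUsed flag locks both ends for three seconds after each jump, preventing an immediate bounce back on arrival.
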(event `self.TeleportCollison1.OnComponentBeginOverlap`
  (params (OverlappedComponent :type "PrimitiveComponent Object Reference") (OtherActor :type "Actor Object Reference") (OtherComp :type "PrimitiveComponent Object Reference") (OtherBodyIndex :type Integer) (bFromSweep :type Boolean) (SweepResult :type "HitResult Structure (by ref)"))
  (bind _teleportcollison2 (`self.TeleportCollison2`))
  (bind _asbp_crystal_player (cast `/Game/Classes/BP_CrystalPlayer` OtherActor))
  (cast `CapsuleComponent` OtherComp)
  (if (`self.canTeleportersBeUsed`)
    (set `self.canTeleportersBeUsed` false)
    (`self.K2_SetActorTransform` _asbp_crystal_player (`KismetMathLibrary.MakeTransform` (`SceneComponent.K2_GetComponentLocation` _teleportcollison2) (`SceneComponent.K2_GetComponentRotation` _teleportcollison2)) false false)
    (`KismetSystemLibrary.Delay` 3.0)
    (set `self.canTeleportersBeUsed` true)))

(event `self.TeleportCollison2.OnComponentBeginOverlap`
  (params (OverlappedComponent :type "PrimitiveComponent Object Reference") (OtherActor :type "Actor Object Reference") (OtherComp :type "PrimitiveComponent Object Reference") (OtherBodyIndex :type Integer) (bFromSweep :type Boolean) (SweepResult :type "HitResult Structure (by ref)"))
  (bind _teleportcollison1 (`self.TeleportCollison1`))
  (bind _asbp_crystal_player (cast `/Game/Classes/BP_CrystalPlayer` OtherActor))
  (cast `CapsuleComponent` OtherComp)
  (if (`self.canTeleportersBeUsed`)
    (set `self.canTeleportersBeUsed` false)
    (`self.K2_SetActorTransform` _asbp_crystal_player (`KismetMathLibrary.MakeTransform` (`SceneComponent.K2_GetComponentLocation` _teleportcollison1) (`SceneComponent.K2_GetComponentRotation` _teleportcollison1)) false false)
    (`KismetSystemLibrary.Delay` 3.0)
    (set `self.canTeleportersBeUsed` true)))

(fn `UserConstructionScript`)