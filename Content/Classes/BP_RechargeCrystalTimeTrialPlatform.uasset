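; Timed platform trial that starts when the crystal player overlaps its trigger, moving the platform to its end point and revealing linked recharge crystals.
; A timeline scaled to the time limit drives two optional HUD countdown reminders and resets the trial on expiry.
; Reset triggers, including an optional leave-area one, return the platform and hide the crystals.
; The finish line stops the timer and arms a safe-to-reset trigger.
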(event `self.ReceiveBeginPlay`
  (bind _asbp_crystal_game_mode (cast `/Game/Classes/BP_CrystalGameMode` (`GameplayStatics.GetGameMode`)))
  (set `self.gameModeReference` _asbp_crystal_game_mode)
  (`SceneComponent.K2_SetWorldLocation` (`self.PlatformCollisionTop`) (`SceneComponent.K2_GetComponentLocation` (`self.StartPoint`)) false false)
  (set `self.platformRelativeRotation` (`SceneComponent.RelativeRotation` (`self.PlatformCollisionTop`)))
  (`SceneComponent.SetVisibility` (`self.ResetTriggerCrystalMesh`) false false)
  (for _array_element (`self.trialRechargeCrystalArray`)
    (`SceneComponent.SetVisibility` (`/Game/Classes/BP_BlastOffRecharge.RechargeCrystalMesh` _array_element) false false)
    (set `PrimitiveComponent.bGenerateOverlapEvents` false (`/Game/Classes/BP_BlastOffRecharge.RechargeCollision` _array_element))
    (if (`self.hasExtraTrigger`)
      (set `PrimitiveComponent.bGenerateOverlapEvents` true (`self.ExtraResetTrigger`))
      (else
        (set `PrimitiveComponent.bGenerateOverlapEvents` false (`self.ExtraResetTrigger`))))))

(event `self.PlatformTrigger.OnComponentBeginOverlap`
  (params (OverlappedComponent :type "PrimitiveComponent Object Reference") (OtherActor :type "Actor Object Reference") (OtherComp :type "PrimitiveComponent Object Reference") (OtherBodyIndex :type Integer) (bFromSweep :type Boolean) (SweepResult :type "HitResult Structure (by ref)"))
  (bind _remindertime2 (`self.reminderTime2`))
  (bind _remindertime1 (`self.reminderTime1`))
  (bind _gamemodehudreference (`/Game/Classes/BP_CrystalGameMode.gameModeHUDReference` (`self.gameModeReference`)))
  (bind _gamemodehudreference_2 (`/Game/Classes/BP_CrystalGameMode.gameModeHUDReference` (`self.gameModeReference`)))
  (bind _gamemodehudreference_3 (`/Game/Classes/BP_CrystalGameMode.gameModeHUDReference` (`self.gameModeReference`)))
  (cast `/Game/Classes/BP_CrystalPlayer` OtherActor)
  (set `self.isTrialHappening` true)
  (set `PrimitiveComponent.bGenerateOverlapEvents` false (`self.PlatformTrigger`))
  (`SceneComponent.SetVisibility` (`self.TriggerCrystalMesh`) false false)
  (`KismetSystemLibrary.MoveComponentTo` (`self.PlatformCollisionTop`) (`SceneComponent.RelativeLocation` (`self.EndPoint`)) (`self.platformRelativeRotation`) false false (`self.destinationTravelTime`))
  (`|ExecutionSequence`
    (:`then_0`
      (`TimelineComponent.SetPlayRate` (`self.TrialTimer`) (/ 1.0 (`self.trialTimeLimit`)))
      (`SceneComponent.SetVisibility` (`self.ResetTriggerCrystalMesh`) true false)
      (set `PrimitiveComponent.bGenerateOverlapEvents` true (`self.PlatformResetTrigger`))
      (`self.ToggleRechargeCrystals` true)
      (bind (_direction _trialtimertrack) (`Timeline|TrialTimer` :!label _label)
        (:`Update`
          (`|ExecutionSequence`
            (:`then_0`
              (if (>= _remindertime1 0.0)
                (bind (_remindertimestring _hasremindertimebeenreached) (`self.TrialReminderMath` _trialtimertrack _remindertime1))
                (if _hasremindertimebeenreached
                  (`/Engine/EditorBlueprintResources/StandardMacros.DoOnce` false :!label _label_2
                    (:`Completed`
                      (`/Game/UI/UIBP_CrystalPlayerHUD.ShowMessagePrompt` _gamemodehudreference_2 _remindertimestring (`self.resetMessageOriginalColor`) true)
                      (`KismetSystemLibrary.Delay` 5.0)
                      (`/Game/UI/UIBP_CrystalPlayerHUD.HideMessagePrompt` _gamemodehudreference_2))))))
            (:`then_1`
              (if (>= _remindertime2 0.0)
                (bind (_remindertimestring_2 _hasremindertimebeenreached_2) (`self.TrialReminderMath` _trialtimertrack _remindertime2))
                (if _hasremindertimebeenreached_2
                  (`/Engine/EditorBlueprintResources/StandardMacros.DoOnce` false :!label _label_3
                    (:`Completed`
                      (`/Game/UI/UIBP_CrystalPlayerHUD.ShowMessagePrompt` _gamemodehudreference_3 _remindertimestring_2 (`self.resetMessageOriginalColor`) true)
                      (`KismetSystemLibrary.Delay` 5.0)
                      (`/Game/UI/UIBP_CrystalPlayerHUD.HideMessagePrompt` _gamemodehudreference_3))))))))
        (:`Finished`
          (`self.ResetTrial`))))
    (:`then_1`
      (`/Game/UI/UIBP_CrystalPlayerHUD.ShowMessagePrompt` _gamemodehudreference (`KismetStringLibrary.Concat_StrStr` (`KismetStringLibrary.Concat_StrStr` "Reach platform origin in " (`KismetStringLibrary.Conv_Int64ToString` (`KismetMathLibrary.Conv_DoubleToInt64` (`self.trialTimeLimit`)))) " seconds") (`self.resetMessageOriginalColor`) true)
      (`KismetSystemLibrary.Delay` 5.0)
      (`/Game/UI/UIBP_CrystalPlayerHUD.HideMessagePrompt` _gamemodehudreference))))

(event `PauseTrial`
  (goto _label :!via `Stop`))

(event `ResetTrial`
  (bind _gamemodehudreference (`/Game/Classes/BP_CrystalGameMode.gameModeHUDReference` (`self.gameModeReference`)))
  (`|ExecutionSequence`
    (:`then_0`
      (goto _label :!via `Stop`))
    (:`then_1`
      (goto _label :!via `SetNewTime`))
    (:`then_2`
      (goto _label_2 :!via `Reset`))
    (:`then_3`
      (goto _label_3 :!via `Reset`))
    (:`then_4`
      (`SceneComponent.SetVisibility` (`self.ResetTriggerCrystalMesh`) false false)
      (set `PrimitiveComponent.bGenerateOverlapEvents` false (`self.PlatformResetTrigger`))
      (`SceneComponent.K2_SetWorldLocation` (`self.PlatformCollisionTop`) (`SceneComponent.K2_GetComponentLocation` (`self.StartPoint`)) false false)
      (`self.ToggleRechargeCrystals` false)
      (`/Game/UI/UIBP_CrystalPlayerHUD.ShowMessagePrompt` _gamemodehudreference (`self.resetMessage`) (`self.resetMessageColor`) true)
      (`KismetSystemLibrary.Delay` 3.0)
      (`/Game/UI/UIBP_CrystalPlayerHUD.HideMessagePrompt` _gamemodehudreference)
      (`SceneComponent.SetVisibility` (`self.TriggerCrystalMesh`) true false)
      (set `PrimitiveComponent.bGenerateOverlapEvents` true (`self.PlatformTrigger`))
      (set `self.resetMessage` "Platform reset")
      (set `PrimitiveComponent.bGenerateOverlapEvents` false (`self.SafeToResetTrigger`))
      (set `self.isTrialHappening` false))))

(event `self.PlatformResetTrigger.OnComponentBeginOverlap`
  (params (OverlappedComponent :type "PrimitiveComponent Object Reference") (OtherActor :type "Actor Object Reference") (OtherComp :type "PrimitiveComponent Object Reference") (OtherBodyIndex :type Integer) (bFromSweep :type Boolean) (SweepResult :type "HitResult Structure (by ref)"))
  (cast `/Game/Classes/BP_CrystalPlayer` OtherActor)
  (`self.ResetTrial` :!label _label_4))

(event `self.ExtraResetTrigger.OnComponentBeginOverlap`
  (params (OverlappedComponent :type "PrimitiveComponent Object Reference") (OtherActor :type "Actor Object Reference") (OtherComp :type "PrimitiveComponent Object Reference") (OtherBodyIndex :type Integer) (bFromSweep :type Boolean) (SweepResult :type "HitResult Structure (by ref)"))
  (if (`self.isTrialHappening`)
    (cast `/Game/Classes/BP_CrystalPlayer` OtherActor)
    (set `self.resetMessage` "Leaving trial area. Platform reset")
    (goto _label_4)))

(event `self.FinishLineTrigger.OnComponentBeginOverlap`
  (params (OverlappedComponent :type "PrimitiveComponent Object Reference") (OtherActor :type "Actor Object Reference") (OtherComp :type "PrimitiveComponent Object Reference") (OtherBodyIndex :type Integer) (bFromSweep :type Boolean) (SweepResult :type "HitResult Structure (by ref)"))
  (bind _gamemodehudreference (`/Game/Classes/BP_CrystalGameMode.gameModeHUDReference` (`self.gameModeReference`)))
  (cast `/Game/Classes/BP_CrystalPlayer` OtherActor)
  (`self.PauseTrial`)
  (set `PrimitiveComponent.bGenerateOverlapEvents` true (`self.SafeToResetTrigger`))
  (`/Game/UI/UIBP_CrystalPlayerHUD.ShowMessagePrompt` _gamemodehudreference "Congratulaions! End reached" (`self.resetMessageOriginalColor`) true)
  (`KismetSystemLibrary.Delay` 3.0)
  (`/Game/UI/UIBP_CrystalPlayerHUD.HideMessagePrompt` _gamemodehudreference))

(event `self.SafeToResetTrigger.OnComponentBeginOverlap`
  (params (OverlappedComponent :type "PrimitiveComponent Object Reference") (OtherActor :type "Actor Object Reference") (OtherComp :type "PrimitiveComponent Object Reference") (OtherBodyIndex :type Integer) (bFromSweep :type Boolean) (SweepResult :type "HitResult Structure (by ref)"))
  (cast `/Game/Classes/BP_CrystalPlayer` OtherActor)
  (`self.ResetTrial`))

(fn `ToggleRechargeCrystals`
  (params (turnOnCrystals :type Boolean))
  (if turnOnCrystals
    (for _array_element (`self.trialRechargeCrystalArray`)
      (`SceneComponent.SetVisibility` (`/Game/Classes/BP_BlastOffRecharge.RechargeCrystalMesh` _array_element) true false)
      (set `PrimitiveComponent.bGenerateOverlapEvents` true (`/Game/Classes/BP_BlastOffRecharge.RechargeCollision` _array_element)))
    (else
      (for _array_element_2 (`self.trialRechargeCrystalArray`)
        (`SceneComponent.SetVisibility` (`/Game/Classes/BP_BlastOffRecharge.RechargeCrystalMesh` _array_element_2) false false)
        (set `PrimitiveComponent.bGenerateOverlapEvents` false (`/Game/Classes/BP_BlastOffRecharge.RechargeCollision` _array_element_2))))))

(fn `TrialReminderMath`
  (params (trialTimerTrack :type "Float (double-precision)") (reminderTime :type "Float (double-precision)"))
  (returns (reminderTimeString :type String) (hasReminderTimeBeenReached :type Boolean))
  (return (`KismetStringLibrary.Concat_StrStr` (`KismetStringLibrary.Conv_Int64ToString` (`KismetMathLibrary.Conv_DoubleToInt64` reminderTime)) " seconds left") (>= (* trialTimerTrack (`self.trialTimeLimit`)) (- (`self.trialTimeLimit`) reminderTime))))

(fn `UserConstructionScript`)